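; BP_DefaultPlayerState is a player state that holds the player's voxel inventory as a map from voxel type data to counts.
; AddVoxels increments or creates a type's entry, then calls the inventory-changed notification, while GetVoxelsNum returns a type's count or zero when absent.
; HandleBreakVoxel adds one voxel of the broken type only when its AddToInventory flag is set, and returns whether it did.
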(fn `AddVoxels`
  (params (InTypeData :type "/Game/Blueprints/World/Voxels/BP_VoxelTypeData Object Reference (by ref)") (InNum :type Integer))
  (bind _intypedata (`local.InTypeData`))
  (bind _inventoryvoxelsnummap (`self.InventoryVoxelsNumMap`))
  (bind (_value _returnvalue) (`BlueprintMapLibrary.Map_Find` (`self.InventoryVoxelsNumMap`) InTypeData))
  (`|ExecutionSequence`
    (:`then_0`
      (if _returnvalue
        (`BlueprintMapLibrary.Map_Add` _inventoryvoxelsnummap _intypedata (+ _value InNum))
        (else
          (`BlueprintMapLibrary.Map_Add` _inventoryvoxelsnummap _intypedata InNum))))
    (:`then_1`
      (`self.NotifyInventoryChanged`))))

(fn `GetVoxelsNum`
  (params (InTypeData :type "/Game/Blueprints/World/Voxels/BP_VoxelTypeData Object Reference (by ref)"))
  (returns (OtNum :type Integer))
  (bind (_value _returnvalue) (`BlueprintMapLibrary.Map_Find` (`self.InventoryVoxelsNumMap`) InTypeData))
  (if _returnvalue
    (return _value)
    (else
      (return 0))))

(fn `HandleBreakVoxel`
  (params (InPoint :type "IntVector Structure") (InTypeData :type "/Game/Blueprints/World/Voxels/BP_VoxelTypeData Object Reference"))
  (returns (bOutAddedToInventory :type Boolean))
  (if (`/Game/Blueprints/World/Voxels/BP_VoxelTypeData.bAddToInventory` InTypeData)
    (`self.AddVoxels` InTypeData 1)
    (return true)
    (else
      (return false))))

(fn `UserConstructionScript`)