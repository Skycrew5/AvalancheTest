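; Test-case voxel chunk that builds preset box shapes in the editor and breaks others at runtime to exercise the voxel system.
; Construction snaps it to the chunk grid, sizes its bounds box and refills voxels from TestVoxelShapes.
; One second after BeginPlay it breaks every point in TestVoxelBreakShapes.
; Debug aids swap voxels for attachment-direction arrows and use the U key to flag marking of stability-update indices.
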(event EventBeginPlay
  (Input|EnableInput (Game|GetPlayerController 0))
  (Utilities|FlowControl|Delay 1.0)
  (for _array_element (Variables|Data|GetTestVoxelBreakShapes)
    (Class|ATVoxelChunk|BreakVoxelsatLocalPoints (CallFunction|GetPointsOfShape _array_element))))

(event Input|KeyboardEvents|DebugKeyU
  (params (Key :type Key%20Structure) (ActionValue :type Input%20Action%20Value%20Structure))
  (:Pressed
    (Utilities|Struct|SetmembersinVoxelChunkPendingUpdates (Variables|Default|GetStabilityUpdates) true false)))

(fn ConstructionScript
  (bind _voxelbasesize (Variables|Default|GetVoxelBaseSize))
  (bind _chunksize (Variables|Default|GetChunkSize))
  (bind _returnvalue (* _chunksize _voxelbasesize))
  (bind _returnvalue_2 (Math|Conversions|ToVector(Float) _returnvalue))
  (bind _returnvalue_3 (* _returnvalue_2 0.5))
  (CallFunction|UpdateDebugAttachments)
  (Transformation|SetActorLocation (Class|KismetMathLibrary|VectorSnappedtoGrid (Transformation|GetActorLocation) (* (Variables|Default|GetChunkSize) (Variables|Default|GetVoxelBaseSize))) false true)
  (Components|Box|SetBoxExtent (Variables|Default|GetBox) _returnvalue_3 false)
  (Transformation|SetRelativeLocation (Variables|Default|GetBox) _returnvalue_3 false false)
  (Class|ATVoxelChunk|ClearAll)
  (for _array_element (Variables|Data|GetTestVoxelShapes)
    (Class|ATVoxelChunk|SetVoxelsatLocalPoints (CallFunction|GetPointsOfShape _array_element) (Variables|Data|GetTestVoxelType))))

(fn GetPointsOfShape
  (params (InShape :type S%20Test%20Case%20Shape%20Structure%20%28by%20ref%29))
  (bind (_start _end) (Utilities|Struct|BreakS_TestCaseShape InShape))
  (bind (_x _y _z) (Utilities|Struct|BreakIntVector _end))
  (bind (_x_2 _y_2 _z_2) (Utilities|Struct|BreakIntVector _start))
  (for _index (range _x_2 _x)
    (for _index_2 (range _y_2 _y)
      (for _index_3 (range _z_2 _z)
        (Utilities|Array|Add (LocalVariables|GetOutPoint) (Utilities|Struct|MakeIntVector _index _index_2 _index_3)))))
  (return (LocalVariables|GetOutPoint)))

(fn UpdateDebugAttachments
  (bind _instancedstaticmeshcomponent (Variables|Default|GetInstancedStaticMeshComponent))
  (if (Variables|Data|GetbDebugAttachements)
    (Components|StaticMesh|SetStaticMesh _instancedstaticmeshcomponent "/Game/Blueprints/World/Voxels/SM_Arrow16x16a.SM_Arrow16x16a")
    (Variables|Default|SetbDebugInstancesAttachmentDirection true)
    (Variables|Default|SetbOffsetMeshToCenter true)
    (else
      (Components|StaticMesh|SetStaticMesh _instancedstaticmeshcomponent "/Game/Blueprints/World/Voxels/SM_Voxel16x16a.SM_Voxel16x16a")
      (Variables|Default|SetbDebugInstancesAttachmentDirection false)
      (Variables|Default|SetbOffsetMeshToCenter false))))