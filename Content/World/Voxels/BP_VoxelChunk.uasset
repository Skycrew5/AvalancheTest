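; BP_VoxelChunk is a world chunk actor that fills a solid cube grid with voxel instances on BeginPlay.
; FillWithVoxels clears its InstancedStaticMesh and transform array, then runs three nested loops sized by the game state's VoxelChunkSize, spacing positions by VoxelSize.
; AddInstances receives the accumulated, uncleared array after each innermost column, so earlier voxels are instanced repeatedly.
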(event `self.ReceiveBeginPlay`
  (`self.FillWithVoxels`))

(fn `FillWithVoxels`
  (locals (VoxelTransforms :type "Array of Transform Structure"))
  (bind _returnvalue (- (`ATGameState.VoxelChunkSize` (`self.Cache_GameState`)) 1))
  (`InstancedStaticMeshComponent.ClearInstances` (`self.InstancedStaticMesh`))
  (`KismetArrayLibrary.Array_Clear` (`local.VoxelTransforms`))
  (for _index (range (+ _returnvalue 1))
    (for _index_2 (range (+ _returnvalue 1))
      (for _index_3 (range (+ _returnvalue 1))
        (`KismetArrayLibrary.Array_Add` (`local.VoxelTransforms`) (`KismetMathLibrary.MakeTransform` (`KismetMathLibrary.MakeVector` (* _index (`self.VoxelSize`)) (* _index_2 (`self.VoxelSize`)) (* _index_3 (`self.VoxelSize`))))))
      (`InstancedStaticMeshComponent.AddInstances` (`self.InstancedStaticMesh`) (`local.VoxelTransforms`) false false true))))

(fn `UserConstructionScript`)