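; Voxel world chunk actor that decides what happens when one of its voxels breaks.
; Two handlers bound to the break event split on the instigator: with one, its BP_DefaultPlayerState handles the voxel for inventory; without one, a BP_BrokenVoxel spawns at that point.
; The construction script snaps the chunk to a grid of chunk size times voxel size and fits its box to those bounds.
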(event `self.ReceiveBeginPlay`
  (add `self.OnBreakVoxelAtPoint` (`|CreateDelegate` :!event `SpawnBrokenVoxel`))
  (add `self.OnBreakVoxelAtPoint` (`|CreateDelegate` :!event `AddVoxelToInstigatorInventory`)))

(event `SpawnBrokenVoxel` :!signature `self.OnBreakVoxelAtPoint`
  (params (InVoxelComponent :type "ATVoxelISMC Object Reference") (InPoint :type "IntVector Structure (by ref)") (InBreakData :type "VoxelBreakData Structure (by ref)"))
  (`/Engine/EditorBlueprintResources/StandardMacros.IsValid` (`.Instigator` (break `VoxelBreakData` InBreakData))
    (:`Is Not Valid`
      (bind _returnvalue (`ATWorldFunctionLibrary.Point3D_To_WorldLocation` InPoint (`self.GetVoxelSize`)))
      (`|SpawnActorFromClass` "/Game/Blueprints/World/Voxels/BP_BrokenVoxel.BP_BrokenVoxel_C" (`KismetMathLibrary.MakeTransform` _returnvalue) "AlwaysSpawn" "MultiplyWithRoot" (`self.GetOwner`) InPoint (`ATVoxelISMC.VoxelTypeData` InVoxelComponent) (`GameplayStatics.GetPlayerPawn` 0)))))

(event `AddVoxelToInstigatorInventory` :!signature `self.OnBreakVoxelAtPoint`
  (params (InVoxelComponent :type "ATVoxelISMC Object Reference") (InPoint :type "IntVector Structure (by ref)") (InBreakData :type "VoxelBreakData Structure (by ref)"))
  (bind ((`Instigator` _instigator)) (break `VoxelBreakData` InBreakData))
  (`/Engine/EditorBlueprintResources/StandardMacros.IsValid` _instigator
    (:`Is Valid`
      (bind _asbp_default_player_state (cast `/Game/Blueprints/Framework/BP_DefaultPlayerState` (`Controller.PlayerState` _instigator)))
      (`/Game/Blueprints/Framework/BP_DefaultPlayerState.HandleBreakVoxel` _asbp_default_player_state InPoint (`.TypeData` (break `VoxelInstanceData` (`ATVoxelTree.GetVoxelInstanceDataAtPoint` (`self.GetOwnerTree`) InPoint true false)))))))

(fn `UserConstructionScript`
  (bind _returnvalue (* (`self.GetChunkSize`) (`self.GetVoxelSize`)))
  (bind _returnvalue_2 (* (`KismetMathLibrary.Conv_DoubleToVector` _returnvalue) 0.5))
  ; Snap to binary grid
  (`self.K2_SetActorLocation` (`KismetMathLibrary.Vector_SnappedToGrid` (`self.K2_GetActorLocation`) _returnvalue) false true)
  (`BoxComponent.SetBoxExtent` (`self.Box`) _returnvalue_2 false)
  (`SceneComponent.K2_SetRelativeLocation` (`self.Box`) _returnvalue_2 false false))