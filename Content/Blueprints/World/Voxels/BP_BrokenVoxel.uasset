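; BP_BrokenVoxel is a loose voxel piece that damages actors it overlaps and resolves itself into the voxel world when it hits something.
; On hit, it converts its location to a grid point and offers it to the instigator's player state to handle.
; If unhandled, it writes its type into the owning voxel tree unless back at its initial point, then destroys itself.
; Overlaps apply type-defined point damage as fall damage.
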(event `self.ReceiveBeginPlay`
  (set `self.OwnerTree` (cast `ATVoxelTree` (`self.GetOwner`) :!pure true)))

(event `self.StaticMesh.OnComponentHit`
  (params (HitComponent :type "PrimitiveComponent Object Reference") (OtherActor :type "Actor Object Reference") (OtherComp :type "PrimitiveComponent Object Reference") (NormalImpulse :type "Vector Structure") (Hit :type "HitResult Structure (by ref)"))
  (bind _returnvalue (`self.GetInstigator`))
  (bind (_x _y _z) (break `IntVector` (`self.InitialPoint`)))
  (bind _returnvalue_2 (* (`ATVoxelTree.GetVoxelSize` (`self.OwnerTree`)) 0.5))
  (bind _returnvalue_3 (+ (`SceneComponent.K2_GetComponentLocation` (`self.StaticMesh`)) _returnvalue_2))
  (`|ExecutionSequence`
    (:`then_0`
      (bind _returnvalue_4 (`ATWorldFunctionLibrary.WorldLocation_To_Point3D` _returnvalue_3 (`ATVoxelTree.GetVoxelSize` (`self.OwnerTree`))))
      (`/Engine/EditorBlueprintResources/StandardMacros.IsValid` _returnvalue
        (:`Is Valid`
          (bind _asbp_default_player_state (cast `/Game/Blueprints/Framework/BP_DefaultPlayerState` (`Pawn.PlayerState` _returnvalue))
            (:`then`
              (bind _boutaddedtoinventory (`/Game/Blueprints/Framework/BP_DefaultPlayerState.HandleBreakVoxel` _asbp_default_player_state _returnvalue_4 (`self.VoxelTypeData`)))
              (if (not _boutaddedtoinventory)
                (bind (_x_2 _y_2 _z_2) (break `IntVector` _returnvalue_4))
                (if (not (and (== _x _x_2) (== _y _y_2) (== _z _z_2))) :!label _label
                  (`ATVoxelTree.SetVoxelAtPoint` (`self.OwnerTree`) _returnvalue_4 (`self.VoxelTypeData`) false))))
            (:`CastFailed`
              (goto _label))))
        (:`Is Not Valid`
          (goto _label))))
    (:`then_1`
      (if (`self.bDrawDebug`)
        (`KismetSystemLibrary.DrawDebugBox` _returnvalue_3 _returnvalue_2 (struct :`R` 1.0 :`A` 1.0) (struct) 4.0 2.0)
        (`KismetSystemLibrary.DrawDebugPoint` _returnvalue_3 8.0 (struct :`G` 1.0 :`A` 1.0) 4.0)))
    (:`then_2`
      (`self.K2_DestroyActor`))))

(event `self.StaticMesh.OnComponentBeginOverlap`
  (params (OverlappedComponent :type "PrimitiveComponent Object Reference") (OtherActor :type "Actor Object Reference") (OtherComp :type "PrimitiveComponent Object Reference") (OtherBodyIndex :type Integer) (bFromSweep :type Boolean) (SweepResult :type "HitResult Structure (by ref)"))
  (`ScWGameplayFunctionLibrary.ApplyPointDamage` self OtherActor (`ATVoxelTypeData.BrokenVoxelLandHitDamage` (`self.VoxelTypeData`)) (`KismetMathLibrary.NegateVector` (`.ImpactNormal` (`GameplayStatics.BreakHitResult` SweepResult))) SweepResult (`self.GetInstigatorController`) "/Game/Blueprints/DamageTypes/BP_VoxelFallDamageType.BP_VoxelFallDamageType_C"))

(fn `UserConstructionScript`)