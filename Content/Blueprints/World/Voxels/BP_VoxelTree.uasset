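; BP_VoxelTree is a voxel tree actor that shows its chunk-based bounds and fades a debug color in voxel materials.
; The construction script sizes a Box from chunk size, voxel size and tree size in chunks, offsetting it so the actor origin sits at a corner.
; Toggling the gameplay debugger plays or reverses a double-speed timeline that writes DebugColorMul to the MPC_VoxelInstance parameter collection.
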(event `self.ReceiveBeginPlay`
  (`TimelineComponent.SetPlayRate` (`self.DebugColorMul change`) 2.0))

(event `self.BP_HandleGameplayDebuggerToggled`
  (params (bInWasActivated :type Boolean))
  (if bInWasActivated
    (bind (_direction _colormul) (`Timeline|DebugColorMul change` :!label _label)
      (:`Update`
        (`KismetMaterialLibrary.SetScalarParameterValue` "/Game/Assets/Materials/MPC_VoxelInstance.MPC_VoxelInstance" "DebugColorMul" _colormul)))
    (else
      (goto _label :!via `Reverse`))))

(fn `UserConstructionScript`
  (bind _returnvalue (* (`KismetMathLibrary.Conv_DoubleToVector` (* (`self.GetChunkSize`) (`self.GetVoxelSize`))) 0.5 (`self.TreeSizeInChunks`)))
  (`BoxComponent.SetBoxExtent` (`self.Box`) _returnvalue false)
  (`SceneComponent.K2_SetRelativeLocation` (`self.Box`) _returnvalue false false))