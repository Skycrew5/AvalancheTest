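; BP_PlayerCharacter is the player character Blueprint, currently handling horizontal movement through Enhanced Input.
; IA_HorizontalMovement feeds AddMovementInput on both Triggered and Completed, mapping X to the actor's right vector and Y to its forward vector.
; Primary and secondary use inputs and possession events are empty stubs, BeginPlay is a disabled default node, and the construction script only calls its parent.
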(event `self.ReceivePossessed`
  (params (NewController :type "Controller Object Reference")))

(event `self.ReceiveUnpossessed`
  (params (OldController :type "Controller Object Reference")))

(event `EnhancedInput|/UnrealCommons/Blueprints/Input/IA_HorizontalMovement`
  (params (ActionValue :type "Vector2D Structure") (ElapsedSeconds :type "Float (double-precision)") (TriggeredSeconds :type "Float (double-precision)") (InputAction :type "InputAction Object Reference" :default "/UnrealCommons/Blueprints/Input/IA_HorizontalMovement.IA_HorizontalMovement"))
  (bind (_x _y) (`KismetMathLibrary.BreakVector2D` ActionValue))
  (:`Triggered`
    (`self.AddMovementInput` (+ (* (`self.GetActorRightVector`) _x) (* (`self.GetActorForwardVector`) _y)) :!label _label))
  (:`Completed`
    (goto _label)))

(event `EnhancedInput|/UnrealCommons/Blueprints/Input/IA_UsePrimary`
  (params (ActionValue :type Boolean) (ElapsedSeconds :type "Float (double-precision)") (TriggeredSeconds :type "Float (double-precision)") (InputAction :type "InputAction Object Reference" :default "/UnrealCommons/Blueprints/Input/IA_UsePrimary.IA_UsePrimary")))

(event `EnhancedInput|/UnrealCommons/Blueprints/Input/IA_UseSecondary`
  (params (ActionValue :type "Float (double-precision)") (ElapsedSeconds :type "Float (double-precision)") (TriggeredSeconds :type "Float (double-precision)") (InputAction :type "InputAction Object Reference" :default "/UnrealCommons/Blueprints/Input/IA_UseSecondary.IA_UseSecondary")))

(fn `UserConstructionScript`
  (`parent.UserConstructionScript`))